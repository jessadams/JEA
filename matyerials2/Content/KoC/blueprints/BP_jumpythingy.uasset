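; BP_jumpythingy is an actor whose static mesh spins and hops repeatedly.
; Tick adds a small world rotation each frame, unscaled by delta time, then runs a two-second Delay.
; When the Delay completes, an upward impulse hits the mesh and Counter is printed.
; A disconnected Counter-based timer for the same impulse never runs.
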(event EventBeginPlay)

(event Collision|EventActorBeginOverlap
  (params (OtherActor :type Actor%20Object%20Reference)))

(event EventTick
  (params (DeltaSeconds :type Float%20%28single-precision%29))
  (Transformation|AddWorldRotation (Variables|Default|GetStaticMesh) "0.150000,0.150000, 0" false false)
  (Utilities|FlowControl|Delay 2.0)
  (Physics|AddImpulse (Variables|Default|GetStaticMesh) "0.000000,0.000000,50000.000000" "None" false)
  (Development|PrintString (Utilities|String|ToString(Float) (stale _output_get))))

(fn ConstructionScript)